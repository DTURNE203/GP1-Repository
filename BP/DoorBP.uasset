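; A locked door Blueprint that opens when the first-person player enters its trigger box while holding at least one key.
; On overlap it reads the Keys count on the player character and spends one key.
; A timeline, DoorAnimation, then drives the relative location of the door mesh to slide it open.
; Leaving the box only performs a cast, so the door never closes.
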(event `self.Box.OnComponentBeginOverlap`
  (params (OverlappedComponent :type "PrimitiveComponent Object Reference") (OtherActor :type "Actor Object Reference") (OtherComp :type "PrimitiveComponent Object Reference") (OtherBodyIndex :type Integer) (bFromSweep :type Boolean) (SweepResult :type "HitResult Structure (by ref)"))
  (bind _as_first_person_character (`self.As First Person Character`))
  (cast `/Game/FirstPersonBP/Blueprints/FirstPersonCharacter` OtherActor)
  (bind _asfirst_person_character (cast `/Game/FirstPersonBP/Blueprints/FirstPersonCharacter` (`GameplayStatics.GetPlayerCharacter` 0)))
  (bind _output_get (set `self.As First Person Character` _asfirst_person_character))
  (if (> (`/Game/FirstPersonBP/Blueprints/FirstPersonCharacter.Keys` _output_get) 0)
    (set `/Game/FirstPersonBP/Blueprints/FirstPersonCharacter.Keys` (- (`/Game/FirstPersonBP/Blueprints/FirstPersonCharacter.Keys` _as_first_person_character) 1) _as_first_person_character)
    (bind (_direction _dooranim) (`Timeline|Door Animation`)
      (:`Update`
        (`SceneComponent.K2_SetRelativeLocation` (`self.Cube`) _dooranim false false)))))

(event `self.Box.OnComponentEndOverlap`
  (params (OverlappedComponent :type "PrimitiveComponent Object Reference") (OtherActor :type "Actor Object Reference") (OtherComp :type "PrimitiveComponent Object Reference") (OtherBodyIndex :type Integer))
  (cast `/Game/FirstPersonBP/Blueprints/FirstPersonCharacter` OtherActor))

(fn `UserConstructionScript`)