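; End-game button actor that loads GameOverLVL and shows the mouse cursor when the player presses Interact nearby.
; Collison overlap with FirstPersonCharacter opens and closes a gate that filters the Interact input.
; A passed press plays timelines lerping Cylinder1 down and back between transforms cached at BeginPlay.
; The level load fires from the press timeline's Update, not on completion.
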(event `self.ReceiveBeginPlay`
  (bind (_returnvalue_location _returnvalue_rotation _returnvalue_scale) (`KismetMathLibrary.BreakTransform` (`SceneComponent.GetRelativeTransform` (`self.Cylinder1`))))
  (set `self.Not Pressed` (`KismetMathLibrary.MakeTransform` _returnvalue_location _returnvalue_rotation _returnvalue_scale))
  (set `self.Pressed` (`KismetMathLibrary.MakeTransform` (- _returnvalue_location (0.0 0.0 10.0)) _returnvalue_rotation _returnvalue_scale))
  (`self.EnableInput` (`GameplayStatics.GetPlayerController` 0)))

(event `self.collison.OnComponentBeginOverlap`
  (params (OverlappedComponent :type "PrimitiveComponent Object Reference") (OtherActor :type "Actor Object Reference") (OtherComp :type "PrimitiveComponent Object Reference") (OtherBodyIndex :type Integer) (bFromSweep :type Boolean) (SweepResult :type "HitResult Structure (by ref)"))
  (cast `/Game/FirstPersonBP/Blueprints/FirstPersonCharacter` OtherActor)
  (goto _label :!via `Open`))

(event `self.collison.OnComponentEndOverlap`
  (params (OverlappedComponent :type "PrimitiveComponent Object Reference") (OtherActor :type "Actor Object Reference") (OtherComp :type "PrimitiveComponent Object Reference") (OtherBodyIndex :type Integer))
  (cast `/Game/FirstPersonBP/Blueprints/FirstPersonCharacter` OtherActor)
  (goto _label :!via `Close`))

(event `InputAction|Interact`
  (params (Key :type "Key Structure"))
  (:`Pressed`
    (`/Engine/EditorBlueprintResources/StandardMacros.Gate` true :!label _label
      (:`Exit`
        (bind (_direction _button_press) (`Timeline|Button Pressed`)
          (:`Update`
            (`SceneComponent.K2_SetRelativeTransform` (`self.Cylinder1`) (`KismetMathLibrary.TLerp` (`self.Not Pressed`) (`self.Pressed`) _button_press) false false)
            (`GameplayStatics.OpenLevel` "GameOverLVL")
            (set `PlayerController.bShowMouseCursor` true (`GameplayStatics.GetPlayerController` 0)))
          (:`Finished`
            (bind (_direction_2 _button_press_2) (`Timeline|Button Out` :!via `ReverseFromEnd`)
              (:`Update`
                (`SceneComponent.K2_SetRelativeTransform` (`self.Cylinder1`) (`KismetMathLibrary.TLerp` (`self.Not Pressed`) (`self.Pressed`) _button_press_2) false false)))))))))

(fn `UserConstructionScript`)